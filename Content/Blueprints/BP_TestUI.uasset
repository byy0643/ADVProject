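; BP_TestUI is a test actor that reveals a widget component when another actor overlaps it.
; The widget starts hidden at BeginPlay.
; On overlap, an enabled Box collision is switched off, a message is logged and the widget is shown.
; If the Box collision is already off, an overlap hides the widget and sets its collision profile to NoCollision.
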(event `self.ReceiveBeginPlay`
  (`SceneComponent.SetVisibility` (`self.Widget`) false false))

(event `self.ReceiveActorBeginOverlap`
  (params (OtherActor :type "Actor Object Reference"))
  (if (`PrimitiveComponent.K2_IsCollisionEnabled` (`self.Box`))
    (`PrimitiveComponent.SetCollisionEnabled` (`self.Box`) "NoCollision")
    (`KismetSystemLibrary.LogString` "Set Collision")
    (`SceneComponent.SetVisibility` (`self.Widget`) true false)
    (else
      (`SceneComponent.SetVisibility` (`self.Widget`) false false)
      (`PrimitiveComponent.SetCollisionProfileName` (`self.Widget`) "NoCollision" true))))

(fn `UserConstructionScript`)