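; BP_Trap is a one-shot spike trap that springs when its Box trigger is overlapped.
; After a short delay it sets TrapUp and rotates the Trap component upright.
; It then calls OnHitEvent on player 0's BP_ADVPlayer, gated by an IsOverlappingActor check that has no actor specified.
; Trap overlap only prints a one-time debug message; TrapBox overlap is empty and the ApplyDamage branch is disconnected.
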(event `self.Box.OnComponentBeginOverlap`
  (params (OverlappedComponent :type "PrimitiveComponent Object Reference") (OtherActor :type "Actor Object Reference") (OtherComp :type "PrimitiveComponent Object Reference") (OtherBodyIndex :type Integer) (bFromSweep :type Boolean) (SweepResult :type "HitResult Structure (by ref)"))
  (`/Engine/EditorBlueprintResources/StandardMacros.DoOnce` false
    (:`Completed`
      (`KismetSystemLibrary.Delay` 0.5)
      (set `self.trapUp` true)
      (`SceneComponent.K2_SetRelativeRotation` (`self.Trap`) (struct :`Roll` 90.0) false false)
      (if (`self.IsOverlappingActor` null)
        (bind _asbp_advplayer (cast `/Game/Blueprints/BP_ADVPlayerUI` (`GameplayStatics.GetPlayerPawn` 0)))
        (`ADVPlayer.OnHitEvent` _asbp_advplayer 60)))))

(event `self.Trap.OnComponentBeginOverlap`
  (params (OverlappedComponent :type "PrimitiveComponent Object Reference") (OtherActor :type "Actor Object Reference") (OtherComp :type "PrimitiveComponent Object Reference") (OtherBodyIndex :type Integer) (bFromSweep :type Boolean) (SweepResult :type "HitResult Structure (by ref)"))
  (`/Engine/EditorBlueprintResources/StandardMacros.DoOnce` false
    (:`Completed`
      (`KismetSystemLibrary.PrintString` "Hitted!"))))

(event `self.TrapBox.OnComponentBeginOverlap`
  (params (OverlappedComponent :type "PrimitiveComponent Object Reference") (OtherActor :type "Actor Object Reference") (OtherComp :type "PrimitiveComponent Object Reference") (OtherBodyIndex :type Integer) (bFromSweep :type Boolean) (SweepResult :type "HitResult Structure (by ref)")))

(fn `UserConstructionScript`)